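; BPC_HealthSystem is a Blueprint component that tracks health and death for its owning actor.
; TakeDamage subtracts from Health, clamps it between zero and MaxHealth, and calls Die when it reaches zero.
; Die runs once behind an IsDead guard, zeroes Health and fires OnDead.
; Kill calls Die directly and then immediately stops the movement component of the owner's Instigator.
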(fn `Die`
  (if (not (`self.IsDead`))
    (set `self.Health` 0.0)
    (set `self.IsDead` true)
    (`self.OnDead`)))

(fn `GetCurrentHealth`
  (returns (Health :type "Float (double-precision)"))
  (return (`self.Health`)))

(fn `GetMaxHealth`
  (returns (MaxHealth :type "Float (double-precision)"))
  (return (`self.MaxHealth`)))

(fn `Kill`
  (`self.Die`)
  (`MovementComponent.StopMovementImmediately` (`Pawn.GetMovementComponent` (`Actor.Instigator` (`self.GetOwner`)))))

(fn `TakeDamage`
  (params (Value :type "Float (double-precision)"))
  (bind _output_get (set `self.Health` (`KismetMathLibrary.FClamp` (- (`self.Health`) Value) 0.0 (`self.MaxHealth`))))
  (if (<= _output_get 0.0)
    (`self.Die`)))