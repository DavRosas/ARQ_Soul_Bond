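; Puzzle terminal actor that lets the player open a puzzle UI when standing inside its trigger volume.
; The trigger tracks the player character's presence and toggles input, so pressing E creates WBP_PuzzleUI with the PuzzleID and terminal reference, or removes an active one.
; Opening shows the cursor and switches to UI-only input; closing does not restore either.
; The solved event only prints a message, and the loop removing WBP_AvisoE widgets is unconnected.
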(event `self.TriggerVolume.OnComponentBeginOverlap`
  (params (OverlappedComponent :type "PrimitiveComponent Object Reference") (OtherActor :type "Actor Object Reference") (OtherComp :type "PrimitiveComponent Object Reference") (OtherBodyIndex :type Integer) (bFromSweep :type Boolean) (SweepResult :type "HitResult Structure (by ref)"))
  (if (== OtherActor (`GameplayStatics.GetPlayerCharacter` 0))
    (set `self.bIsPlayerInRange` true)
    (`self.EnableInput` (`GameplayStatics.GetPlayerController` 0))))

(event `self.TriggerVolume.OnComponentEndOverlap`
  (params (OverlappedComponent :type "PrimitiveComponent Object Reference") (OtherActor :type "Actor Object Reference") (OtherComp :type "PrimitiveComponent Object Reference") (OtherBodyIndex :type Integer))
  (if (== OtherActor (`GameplayStatics.GetPlayerCharacter` 0))
    (set `self.bIsPlayerInRange` false)
    (`self.DisableInput` (`GameplayStatics.GetPlayerController` 0))))

(event `Key|E`
  (params (Key :type "Key Structure"))
  (bind _returnvalue (`GameplayStatics.GetPlayerController` 0))
  (:`Pressed`
    (if (`self.bIsPlayerInRange`)
      (if (`KismetSystemLibrary.IsValid` (`self.ActivePuzzleUI`))
        (`Widget.RemoveFromParent` (`self.ActivePuzzleUI`))
        (set `self.ActivePuzzleUI` null)
        (else
          (bind _returnvalue_2 (`|CreateWidget` "/Game/Gameplay/Puzzles/WBP_PuzzleUI.WBP_PuzzleUI_C" (`GameplayStatics.GetPlayerController` 0) (`self.PuzzleID`) self))
          (`UserWidget.AddToViewport` _returnvalue_2 0)
          (bind _foundwidgets (`WidgetBlueprintLibrary.GetAllWidgetsOfClass` "/Game/UI/HUD/AvisosInteracccion/WBP_AvisoE.WBP_AvisoE_C" false))
          (set `self.ActivePuzzleUI` _returnvalue_2)
          (set `PlayerController.bShowMouseCursor` true _returnvalue)
          (`WidgetBlueprintLibrary.SetInputMode_UIOnlyEx` _returnvalue _returnvalue_2))))))

(event `Event_OnPuzzleSolved`
  (`KismetSystemLibrary.PrintString` "Puzzle Resuelto"))

(fn `UserConstructionScript`)