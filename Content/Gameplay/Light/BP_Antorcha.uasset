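; BP_Antorcha is a torch pickup with a flame and a light set by exposed intensity and radius.
; CubeRecoger overlaps register it as BP_ThirdPersonCharacter's nearby torch and toggle the prompt widget; leaving keeps that reference rather than clearing it.
; AlRecoger disables physics and collision, while AlSoltar restores them with a downward impulse.
; SetEscondida hides or shows actor, light and flame.
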(event `self.CubeRecoger.OnComponentBeginOverlap`
  (params (OverlappedComponent :type "PrimitiveComponent Object Reference") (OtherActor :type "Actor Object Reference") (OtherComp :type "PrimitiveComponent Object Reference") (OtherBodyIndex :type Integer) (bFromSweep :type Boolean) (SweepResult :type "HitResult Structure (by ref)"))
  (bind _asbp_third_person_character (cast `/Game/Characters/Player/BP_ThirdPersonCharacter` OtherActor))
  (set `/Game/Characters/Player/BP_ThirdPersonCharacter.AntorchaCercana` self _asbp_third_person_character)
  (`/Game/Gameplay/Interaction/BPI_Interaccion.MostrarWidget` _asbp_third_person_character))

(event `self.CubeRecoger.OnComponentEndOverlap`
  (params (OverlappedComponent :type "PrimitiveComponent Object Reference") (OtherActor :type "Actor Object Reference") (OtherComp :type "PrimitiveComponent Object Reference") (OtherBodyIndex :type Integer))
  (bind _asbp_third_person_character (cast `/Game/Characters/Player/BP_ThirdPersonCharacter` OtherActor))
  (if (== self (`/Game/Characters/Player/BP_ThirdPersonCharacter.AntorchaCercana` _asbp_third_person_character))
    (set `/Game/Characters/Player/BP_ThirdPersonCharacter.AntorchaCercana` self _asbp_third_person_character)
    (`/Game/Gameplay/Interaction/BPI_Interaccion.OcultarWidget` _asbp_third_person_character)))

(fn `AlRecoger`
  (`PrimitiveComponent.SetSimulatePhysics` (`self.MallaAntorcha`) false)
  (`PrimitiveComponent.SetCollisionEnabled` (`self.CubeRecoger`) "NoCollision")
  (`PrimitiveComponent.SetCollisionEnabled` (`self.MallaAntorcha`) "NoCollision"))

(fn `AlSoltar`
  (`self.SetActorEnableCollision` true)
  (`PrimitiveComponent.SetCollisionEnabled` (`self.MallaAntorcha`) "QueryAndPhysics")
  (`PrimitiveComponent.SetCollisionEnabled` (`self.CubeRecoger`) "QueryOnly")
  (`PrimitiveComponent.SetSimulatePhysics` (`self.MallaAntorcha`) true)
  (`PrimitiveComponent.WakeRigidBody` (`self.MallaAntorcha`) "None")
  (`PrimitiveComponent.AddImpulse` (`self.MallaAntorcha`) (0.0 0.0 -100.0) "None" true))

(fn `SetEscondida`
  (params (Escondida :type Boolean))
  (bind _returnvalue (not Escondida))
  (`self.SetActorHiddenInGame` Escondida)
  (`SceneComponent.SetVisibility` (`self.LuzAntorcha`) _returnvalue true)
  (`SceneComponent.SetVisibility` (`self.Llama`) _returnvalue true))

(fn `UserConstructionScript`
  (`LightComponent.SetIntensity` (`self.LuzAntorcha`) (`self.IntensidadLuz`))
  (`LocalLightComponent.SetAttenuationRadius` (`self.LuzAntorcha`) (`self.RadioLuz`)))