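; BP_ZonaCamara is a camera zone that switches the view to its own camera while the player pawn is inside its box.
; On overlap it saves the camera's pose, blends the view to itself, and each Tick follows the player at the camera's offset from the zone with fixed rotation.
; On exit it restores that pose and blends back to the pawn.
; The construction logic placing the camera from Distancia and Altura is disconnected.
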(event `self.ReceiveTick`
  (params (DeltaSeconds :type "Float (single-precision)"))
  (bind _camarazona (`self.CamaraZona`))
  (if (`self.Siguiendo`)
    (`SceneComponent.K2_SetWorldLocation` _camarazona (+ (`self.Offset`) (`self.K2_GetActorLocation` (`GameplayStatics.GetPlayerPawn` 0))) false false)
    (`SceneComponent.K2_SetWorldRotation` _camarazona (`self.RotacionCamara`) false false)))

(event `self.CajaZona.OnComponentBeginOverlap`
  (params (OverlappedComponent :type "PrimitiveComponent Object Reference") (OtherActor :type "Actor Object Reference") (OtherComp :type "PrimitiveComponent Object Reference") (OtherBodyIndex :type Integer) (bFromSweep :type Boolean) (SweepResult :type "HitResult Structure (by ref)"))
  (if (== OtherActor (`GameplayStatics.GetPlayerPawn` 0))
    (set `self.JugadorDentro` true)
    (set `self.RelLocGuardada` (`SceneComponent.RelativeLocation` (`self.CamaraZona`)))
    (set `self.RelRotGuardada` (`SceneComponent.RelativeRotation` (`self.CamaraZona`)))
    (set `self.RotacionCamara` (`SceneComponent.K2_GetComponentRotation` (`self.CamaraZona`)))
    (set `self.Offset` (- (`SceneComponent.K2_GetComponentLocation` (`self.CamaraZona`)) (`self.K2_GetActorLocation`)))
    (set `self.Siguiendo` true)
    (`PlayerController.SetViewTargetWithBlend` (`GameplayStatics.GetPlayerController` 0) self 0.3 "VTBlend_EaseInOut" 0.0 true)))

(event `self.CajaZona.OnComponentEndOverlap`
  (params (OverlappedComponent :type "PrimitiveComponent Object Reference") (OtherActor :type "Actor Object Reference") (OtherComp :type "PrimitiveComponent Object Reference") (OtherBodyIndex :type Integer))
  (bind _returnvalue (`GameplayStatics.GetPlayerPawn` 0))
  (if (== OtherActor _returnvalue)
    (set `self.Siguiendo` false)
    (`SceneComponent.K2_SetRelativeLocation` (`self.CamaraZona`) (`self.RelLocGuardada`) false false)
    (`SceneComponent.K2_SetRelativeRotation` (`self.CamaraZona`) (`self.RelRotGuardada`) false false)
    (`PlayerController.SetViewTargetWithBlend` (`GameplayStatics.GetPlayerController` 0) _returnvalue 0.3 "VTBlend_EaseInOut" 0.0 true)))

(fn `UserConstructionScript`)