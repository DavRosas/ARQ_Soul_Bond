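; BP_LevelExit is a level exit that unlocks and wins the game when the player's currency equals three.
; It binds to the player's BP_CurrencyComponent change event and disables BlockingBox collision at that exact count.
; WinTrigger rechecks the count when a BP_ThirdPersonCharacter overlaps it.
; Win runs once, broadcasting OnWon and showing UI_Victory with UI-only input and a mouse cursor.
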(event `self.ReceiveBeginPlay`
  (set `self.PlayerCurrency` (`self.GetComponentByClass` (`GameplayStatics.GetPlayerCharacter` 0) "/Game/Gameplay/Currency_System/BP_CurrencyComponent.BP_CurrencyComponent_C"))
  (add `/Game/Gameplay/Currency_System/BP_CurrencyComponent.OnCurrencyChanged` (`self.PlayerCurrency`) (delegate `HandleCurrencyChanged`)))

(event `HandleCurrencyChanged`
  (params (Amount :type Integer))
  (if (== 3 (`/Game/Gameplay/Currency_System/BP_CurrencyComponent.Currency` (`self.PlayerCurrency`)))
    (`PrimitiveComponent.SetCollisionEnabled` (`self.BlockingBox`) "NoCollision")))

(event `self.WinTrigger.OnComponentBeginOverlap`
  (params (OverlappedComponent :type "PrimitiveComponent Object Reference") (OtherActor :type "Actor Object Reference") (OtherComp :type "PrimitiveComponent Object Reference") (OtherBodyIndex :type Integer) (bFromSweep :type Boolean) (SweepResult :type "HitResult Structure (by ref)"))
  (cast `/Game/Characters/Player/BP_ThirdPersonCharacter` OtherActor)
  (if (== (`/Game/Gameplay/Currency_System/BP_CurrencyComponent.Currency` (`self.PlayerCurrency`)) 3)
    (`self.Win`)))

(fn `UserConstructionScript`)

(fn `Win`
  (bind _returnvalue (`GameplayStatics.GetPlayerController` 0))
  (if (not (`self.IsWon`))
    (set `self.IsWon` true)
    (`self.OnWon`)
    (bind _returnvalue_2 (`|CreateWidget` "/Game/UI/UI_Currency/UI_Victory.UI_Victory_C" _returnvalue))
    (`UserWidget.AddToViewport` _returnvalue_2 0)
    (`WidgetBlueprintLibrary.SetInputMode_UIOnlyEx` _returnvalue _returnvalue_2)
    (set `PlayerController.bShowMouseCursor` true (`GameplayStatics.GetPlayerController` 0))))