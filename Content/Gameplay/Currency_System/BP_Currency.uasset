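; BP_Currency is a currency pickup that bobs on a sine wave until collected.
; On sphere overlap with an actor owning BP_CurrencyComponent, it disables collision, adds Amount and plays sounds, including Fondo_Terremoto.
; Tick then raises and shrinks the actor, destroying it within a fraction of a second.
; The five-second delayed sound fade, glow and spin boost sit behind that destruction, so likely never run.
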(event `self.ReceiveTick`
  (params (DeltaSeconds :type "Float (single-precision)"))
  (bind _returnvalue (- (.x (`self.GetActorScale3D`)) (* DeltaSeconds 4.0)))
  (if (`self.Recogida`)
    (`self.K2_AddActorWorldOffset` (`KismetMathLibrary.MakeVector` 0.0 0.0 (* DeltaSeconds 250.0)))
    (if (<= _returnvalue 0.05)
      (`self.K2_DestroyActor`)
      (else
        (`self.SetActorScale3D` (`KismetMathLibrary.MakeVector` _returnvalue _returnvalue _returnvalue))))
    (else
      (`SceneComponent.K2_SetRelativeLocation` (`self.StaticMesh`) (`KismetMathLibrary.MakeVector` 0.0 0.0 (* (`KismetMathLibrary.Sin` (* (`KismetSystemLibrary.GetGameTimeInSeconds`) 3.0)) 8.0)) false false))))

(event `self.Sphere.OnComponentBeginOverlap`
  (params (OverlappedComponent :type "PrimitiveComponent Object Reference") (OtherActor :type "Actor Object Reference") (OtherComp :type "PrimitiveComponent Object Reference") (OtherBodyIndex :type Integer) (bFromSweep :type Boolean) (SweepResult :type "HitResult Structure (by ref)"))
  (bind _returnvalue (`self.GetComponentByClass` OtherActor "/Game/Gameplay/Currency_System/BP_CurrencyComponent.BP_CurrencyComponent_C"))
  (if (not (`self.Recogida`))
    (`/Engine/EditorBlueprintResources/StandardMacros.IsValid` _returnvalue
      (:`Is Valid`
        (set `self.Recogida` true)
        (`self.SetActorEnableCollision` false)
        (`/Game/Gameplay/Currency_System/BP_CurrencyComponent.Add Currency` _returnvalue (`self.Amount`))
        (`GameplayStatics.SpawnSound2D` null 1.0 1.0 0.0 null false false)
        (bind _returnvalue_2 (`GameplayStatics.SpawnSound2D` "/Game/Audio/Ambient/Fondo_Terremoto.Fondo_Terremoto" 1.0 1.0 0.0 null false false))
        (set `self.AudioTerremoto` _returnvalue_2)
        (`KismetSystemLibrary.Delay` 5.0)
        (`AudioComponent.FadeOut` _returnvalue_2 0.2 0.0 "Linear")
        (`AudioComponent.Stop` _returnvalue_2)
        (`self.K2_DestroyActor`)
        (`LightComponent.SetIntensity` (`self.Brillo`) 40.0)
        (set `RotatingMovementComponent.RotationRate` (`KismetMathLibrary.MakeRotator` 0.0 0.0 720.0) (`self.Giro`))))))

(fn `UserConstructionScript`)