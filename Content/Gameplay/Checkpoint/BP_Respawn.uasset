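; BP_Respawn is a trigger box that revives the third-person character when it overlaps.
; With a valid LastCheckPoint, it clears the death flags and refills health through the health component, but does not move the character.
; Without one, it clears EstaMuerto and teleports the character to its SpawnTransform, raised by capsule half-height, leaving health untouched.
; The checkpoint location lookup is unwired, and a set-property-by-name call has no property name.
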(event `self.Box.OnComponentBeginOverlap`
  (params (OverlappedComponent :type "PrimitiveComponent Object Reference") (OtherActor :type "Actor Object Reference") (OtherComp :type "PrimitiveComponent Object Reference") (OtherBodyIndex :type Integer) (bFromSweep :type Boolean) (SweepResult :type "HitResult Structure (by ref)"))
  (bind _bpc_healthsystem (`self.BPC_HealthSystem`))
  (bind _asbp_third_person_character (cast `/Game/Characters/Player/BP_ThirdPersonCharacter` OtherActor))
  (bind _lastcheckpoint (`/Game/Characters/Player/BP_ThirdPersonCharacter.LastCheckPoint` _asbp_third_person_character)
    (:`then`
      (set `/Game/Characters/Player/BP_ThirdPersonCharacter.bEstaMuerto` false _asbp_third_person_character)
      (`KismetSystemLibrary.SetIntPropertyByName` (`self.GetComponentByClass` _asbp_third_person_character "/Game/Gameplay/Health/BPC_HealthSystem.BPC_HealthSystem_C") "None" 1)
      (set `/Game/Gameplay/Health/BPC_HealthSystem.Health` (`/Game/Gameplay/Health/BPC_HealthSystem.MaxHealth` _bpc_healthsystem) _bpc_healthsystem)
      (set `/Game/Gameplay/Health/BPC_HealthSystem.IsDead` false _bpc_healthsystem))
    (:`else`
      (set `/Game/Characters/Player/BP_ThirdPersonCharacter.bEstaMuerto` false _asbp_third_person_character)
      (bind (_spawntransform_location _spawntransform_rotation) (`KismetMathLibrary.BreakTransform` (`/Game/Characters/Player/BP_ThirdPersonCharacter.SpawnTransform` _asbp_third_person_character)))
      (`self.K2_SetActorLocationAndRotation` _asbp_third_person_character (`KismetMathLibrary.MakeVector` (.x _spawntransform_location) (.y _spawntransform_location) (+ (.z _spawntransform_location) (`CapsuleComponent.GetScaledCapsuleHalfHeight` (`Character.CapsuleComponent` _asbp_third_person_character)))) _spawntransform_rotation false true))))

(event `self.ReceiveActorBeginOverlap`
  (params (OtherActor :type "Actor Object Reference")))

(fn `UserConstructionScript`)