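; BP_Escalera is a ladder actor whose climbing zone restricts torch use for the third-person character.
; Entering ZonaEscalada clears the character's PuedeUsarAntorcha flag and, if a torch is equipped, plays an error sound and shows the character's warning widget text.
; Leaving the zone restores the flag and hides the warning.
; The Blueprint contains no climbing movement logic, only these overlap responses.
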(event `self.ZonaEscalada.OnComponentBeginOverlap`
  (params (OverlappedComponent :type "PrimitiveComponent Object Reference") (OtherActor :type "Actor Object Reference") (OtherComp :type "PrimitiveComponent Object Reference") (OtherBodyIndex :type Integer) (bFromSweep :type Boolean) (SweepResult :type "HitResult Structure (by ref)"))
  (bind _asbp_third_person_character (cast `/Game/Characters/Player/BP_ThirdPersonCharacter` OtherActor))
  (set `/Game/Characters/Player/BP_ThirdPersonCharacter.PuedeUsarAntorcha` false _asbp_third_person_character)
  (if (`KismetSystemLibrary.IsValid` (`/Game/Characters/Player/BP_ThirdPersonCharacter.AntorchaEquipada` _asbp_third_person_character))
    (`GameplayStatics.PlaySound2D` "/Game/Audio/error.error" 5.0 1.0 0.0 null null)
    (`/Game/UI/HUD/AvisosInteracccion/WBP_Aviso_Escaleras.MostrarTexto` (`/Game/Characters/Player/BP_ThirdPersonCharacter.WidgetAviso` _asbp_third_person_character))))

(event `self.ZonaEscalada.OnComponentEndOverlap`
  (params (OverlappedComponent :type "PrimitiveComponent Object Reference") (OtherActor :type "Actor Object Reference") (OtherComp :type "PrimitiveComponent Object Reference") (OtherBodyIndex :type Integer))
  (bind _asbp_third_person_character (cast `/Game/Characters/Player/BP_ThirdPersonCharacter` OtherActor))
  (set `/Game/Characters/Player/BP_ThirdPersonCharacter.PuedeUsarAntorcha` true _asbp_third_person_character)
  (`/Game/UI/HUD/AvisosInteracccion/WBP_Aviso_Escaleras.OcultarTexto_` (`/Game/Characters/Player/BP_ThirdPersonCharacter.WidgetAviso` _asbp_third_person_character)))

(fn `UserConstructionScript`)