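; BP_BloqueMensaje is a message block actor in the DevRoom folder that displays a title and body text.
; The construction script writes Titulo and Mensaje into the TextoTitulo and TextoCuerpo components.
; At BeginPlay, ActualizarMensaje creates a WBP_MensajeBloque, passes it the same strings and assigns it to the Widget component.
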(event `self.ReceiveBeginPlay`
  (`self.ActualizarMensaje`))

(fn `ActualizarMensaje`
  (bind _returnvalue (`|CreateWidget` "/Game/UI/Mensajes_DevRoom/WBP_MensajeBloque.WBP_MensajeBloque_C"))
  (`/Game/UI/Mensajes_DevRoom/WBP_MensajeBloque.EstablecerMensaje` _returnvalue (`self.Titulo`) (`self.Mensaje`))
  (`WidgetComponent.SetWidget` (`self.Widget`) _returnvalue))

(fn `UserConstructionScript`
  (`TextRenderComponent.K2_SetText` (`self.Texto Titulo`) (`self.Titulo`))
  (`TextRenderComponent.K2_SetText` (`self.Texto Cuerpo`) (`self.Mensaje`)))