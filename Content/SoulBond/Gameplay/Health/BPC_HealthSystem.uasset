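; BPC_HealthSystem is a health component that stores health, max health and a death flag.
; TakeDamage subtracts the given value, clamps the result between zero and MaxHealth, and sets IsDead when health runs out.
; Getters expose current and maximum health, while the event graph is inactive and no event is broadcast on damage or death.
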(fn `GetCurrentHealth`
  (returns (Health :type "Float (double-precision)"))
  (return (`self.Health`)))

(fn `GetMaxHealth`
  (returns (MaxHealth :type "Float (double-precision)"))
  (return (`self.MaxHealth`)))

(fn `TakeDamage`
  (params (Value :type "Float (double-precision)"))
  (bind _output_get (set `self.Health` (`KismetMathLibrary.FClamp` (- (`self.Health`) Value) 0.0 (`self.MaxHealth`))))
  (if (<= _output_get 0.0)
    (set `self.IsDead` true)))