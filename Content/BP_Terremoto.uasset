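; BP_Terremoto is an actor that triggers recurring random earthquakes for the first player.
; From BeginPlay, a self-calling event waits a random delay, then picks a random strength and duration.
; The strength drives both the earthquake audio volume and the scale of the CS_Terremoto camera shake.
; When the duration ends it stops the audio and shake, then schedules the next quake.
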(event `self.ReceiveBeginPlay`
  (`self.DispararTerremoto`))

(event `DispararTerremoto`
  (`KismetSystemLibrary.Delay` (`KismetMathLibrary.RandomFloatInRange` 10.0 35.0))
  (set `self.Fuerza` (`KismetMathLibrary.RandomFloatInRange` 1.0 4.0))
  (set `self.Duracion` (`KismetMathLibrary.RandomFloatInRange` 4.0 12.0))
  (`AudioComponent.SetVolumeMultiplier` (`self.AudioTerremoto`) (`self.Fuerza`))
  (`AudioComponent.Play` (`self.AudioTerremoto`) 0.0)
  (`PlayerController.ClientStartCameraShake` :`self` (`GameplayStatics.GetPlayerController` 0) :`Shake` "/Game/CS_Terremoto.CS_Terremoto_C" :`Scale` (`self.Fuerza`))
  (`KismetSystemLibrary.Delay` (`self.Duracion`))
  (`AudioComponent.Stop` (`self.AudioTerremoto`))
  (`PlayerController.ClientStopCameraShake` (`GameplayStatics.GetPlayerController` 0) "/Game/CS_Terremoto.CS_Terremoto_C" false)
  (`self.DispararTerremoto`))

(fn `UserConstructionScript`)