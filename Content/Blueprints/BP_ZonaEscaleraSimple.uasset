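; Simple ladder zone that lets the player climb while overlapping it, toggled with either Shift key.
; Tick polls the keys with edge detection, switching CharacterMovement off and zeroing gravity to climb, or restoring both to exit.
; While climbing, W and S move the player along the zone's up vector at fixed speed, using unswept teleport offsets.
; Any end overlap restores normal movement and clears the climbing state.
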(event `self.ReceiveActorEndOverlap`
  (params (OtherActor :type "Actor Object Reference"))
  (bind _ascharacter_movement_component (cast `CharacterMovementComponent` (`self.GetComponentByClass` (`GameplayStatics.GetPlayerCharacter` 0) "/Script/Engine.CharacterMovementComponent") :!pure true))
  (`ActorComponent.SetActive` _ascharacter_movement_component true false)
  (`KismetSystemLibrary.PrintString` "salir")
  (set `CharacterMovementComponent.GravityScale` 1.0 _ascharacter_movement_component)
  (set `CharacterMovementComponent.AirControl` 0.05 _ascharacter_movement_component)
  (set `self.bIsClimbing` false))

(event `self.ReceiveTick`
  (params (DeltaSeconds :type "Float (single-precision)"))
  (bind _returnvalue (`GameplayStatics.GetPlayerCharacter` 0))
  (bind _returnvalue_2 (`GameplayStatics.GetPlayerController` 0))
  (bind _returnvalue_3 (or (`PlayerController.IsInputKeyDown` _returnvalue_2 "LeftShift") (`PlayerController.IsInputKeyDown` _returnvalue_2 "RightShift")))
  (bind _ascharacter_movement_component (cast `CharacterMovementComponent` (`self.GetComponentByClass` _returnvalue "/Script/Engine.CharacterMovementComponent") :!pure true))
  (`|ExecutionSequence`
    (:`then_0`
      (if (and (and _returnvalue_3 (not (`self.bShiftWasDown`))) (`self.IsOverlappingActor` self _returnvalue))
        (if (`self.bIsClimbing`)
          (`ActorComponent.SetActive` _ascharacter_movement_component true false)
          (`KismetSystemLibrary.PrintString` "salir")
          (set `CharacterMovementComponent.GravityScale` 1.0 _ascharacter_movement_component)
          (set `CharacterMovementComponent.AirControl` 0.05 _ascharacter_movement_component)
          (set `self.bIsClimbing` false)
          (else
            (`ActorComponent.SetActive` _ascharacter_movement_component false false)
            (`KismetSystemLibrary.PrintString` "entrar")
            (set `CharacterMovementComponent.GravityScale` 0.0 _ascharacter_movement_component)
            (set `CharacterMovementComponent.AirControl` 1.0 _ascharacter_movement_component)
            (set `self.bIsClimbing` true)))))
    (:`then_1`
      (set `self.bShiftWasDown` _returnvalue_3)
      (if (`self.bIsClimbing`)
        (`self.K2_AddActorWorldOffset` _returnvalue (* (`self.GetActorUpVector` self) (* (* (+ (`KismetMathLibrary.SelectFloat` 1.0 0.0 (`PlayerController.IsInputKeyDown` _returnvalue_2 "W")) (`KismetMathLibrary.SelectFloat` -1.0 0.0 (`PlayerController.IsInputKeyDown` _returnvalue_2 "S"))) 250.0) DeltaSeconds)) false true)))))

(fn `UserConstructionScript`)