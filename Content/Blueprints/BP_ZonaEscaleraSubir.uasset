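; BP_ZonaEscaleraSubir is a ladder climb zone that moves the player up and down.
; On any overlap begin it deactivates the player's CharacterMovementComponent and zeroes gravity, restoring both on overlap end, without checking which actor overlapped.
; Each Tick polls W and S directly and, while the player overlaps, teleports them unswept along the zone's up vector at a fixed speed.
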(event `self.ReceiveActorBeginOverlap`
  (params (OtherActor :type "Actor Object Reference"))
  (bind _ascharacter_movement_component (cast `CharacterMovementComponent` (`self.GetComponentByClass` (`GameplayStatics.GetPlayerCharacter` 0) "/Script/Engine.CharacterMovementComponent")))
  (`ActorComponent.SetActive` _ascharacter_movement_component false false)
  (`KismetSystemLibrary.PrintString` "entrar")
  (set `CharacterMovementComponent.GravityScale` 0.0 _ascharacter_movement_component))

(event `self.ReceiveActorEndOverlap`
  (params (OtherActor :type "Actor Object Reference"))
  (bind _ascharacter_movement_component (cast `CharacterMovementComponent` (`self.GetComponentByClass` (`GameplayStatics.GetPlayerCharacter` 0) "/Script/Engine.CharacterMovementComponent")))
  (`ActorComponent.SetActive` _ascharacter_movement_component true false)
  (set `CharacterMovementComponent.GravityScale` 1.0 _ascharacter_movement_component))

(event `self.ReceiveTick`
  (params (DeltaSeconds :type "Float (single-precision)"))
  (bind _returnvalue (`GameplayStatics.GetPlayerCharacter` 0))
  (bind _returnvalue_2 (`GameplayStatics.GetPlayerController` 0))
  (`self.K2_AddActorWorldOffset` _returnvalue (* (`self.GetActorUpVector` self) (* (* (* (+ (`KismetMathLibrary.SelectFloat` 1.0 0.0 (`PlayerController.IsInputKeyDown` _returnvalue_2 "W")) (`KismetMathLibrary.SelectFloat` -1.0 0.0 (`PlayerController.IsInputKeyDown` _returnvalue_2 "S"))) (`KismetMathLibrary.SelectFloat` 1.0 0.0 (`self.IsOverlappingActor` self _returnvalue))) 250.0) DeltaSeconds)) false true))

(fn `UserConstructionScript`)