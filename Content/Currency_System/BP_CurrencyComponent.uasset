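; BP_CurrencyComponent is a component that holds a Currency balance and shows it on screen.
; On BeginPlay it creates a UI_Currency widget, adds it to the viewport and displays the starting balance.
; AddCurrency and SpendCurrency adjust the balance and fire the OnCurrencyChanged dispatcher, which the component binds to refresh the widget.
; SpendCurrency subtracts without checking that the balance covers the amount.
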(event `self.ReceiveBeginPlay`
  (bind _returnvalue (`|CreateWidget` "/Game/Currency_System/UI_Currency.UI_Currency_C"))
  (bind _output_get (set `self.Widget` _returnvalue))
  (`UserWidget.AddToViewport` _output_get 0)
  (`/Game/Currency_System/UI_Currency.Update Currency` (`self.Widget`) (`self.Currency`))
  (add `self.OnCurrencyChanged` (delegate `Update Currency`)))

(event `Update Currency` :!signature `self.OnCurrencyChanged`
  (params (Amount :type Integer))
  (`/Game/Currency_System/UI_Currency.Update Currency` (`self.Widget`) Amount))

(fn `Add Currency`
  (params (Amount :type Integer))
  (bind _output_get (set `self.Currency` (+ Amount (`self.Currency`))))
  (`self.OnCurrencyChanged` _output_get))

(fn `Spend Currency`
  (params (Amount :type Integer))
  (bind _output_get (set `self.Currency` (- (`self.Currency`) Amount)))
  (`self.OnCurrencyChanged` _output_get))